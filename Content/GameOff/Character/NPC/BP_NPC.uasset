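; NPC character that gets squashed and killed on being hit, leaving a Bone pickup or prop behind.
; A capsule hit from an actor with upward velocity disables collision, stops movement and flattens the mesh vertically.
; A short timer then fires Killed, which plays an explosion effect, destroys the NPC and spawns a Bone at its XY location and a fixed height.
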(event `self.ReceiveBeginPlay`)

(event `self.CapsuleComponent.OnComponentHit`
  (params (HitComponent :type "PrimitiveComponent Object Reference") (OtherActor :type "Actor Object Reference") (OtherComp :type "PrimitiveComponent Object Reference") (NormalImpulse :type "Vector Structure") (Hit :type "HitResult Structure (by ref)"))
  (bind _mesh (`self.Mesh`))
  (bind (_returnvalue_x _returnvalue_y _returnvalue_z) (`KismetMathLibrary.BreakVector` (`KismetMathLibrary.Normal` (`self.GetVelocity` OtherActor))))
  (bind (_relativescale3d_x _relativescale3d_y _relativescale3d_z) (`KismetMathLibrary.BreakVector` (`SceneComponent.RelativeScale3D` _mesh)))
  (if (> _returnvalue_z 0.0)
    (`PrimitiveComponent.SetCollisionEnabled` (`self.CapsuleComponent`) "NoCollision")
    (`NavMovementComponent.StopActiveMovement` (`self.CharacterMovement`))
    (`SceneComponent.SetRelativeScale3D` _mesh (`KismetMathLibrary.MakeVector` _relativescale3d_x _relativescale3d_y (/ _relativescale3d_z 1.5)))
    (`SceneComponent.K2_AddLocalOffset` _mesh (0.0 0.0 0.0) false true)
    (`KismetSystemLibrary.K2_SetTimerDelegate` (delegate `Killed`) 0.5)))

(event `Killed`
  (bind (_returnvalue_x _returnvalue_y) (`KismetMathLibrary.BreakVector` (`self.K2_GetActorLocation`)))
  (`NiagaraFunctionLibrary.SpawnSystemAtLocation` "/Niagara/DefaultAssets/Templates/Systems/SimpleExplosion.SimpleExplosion" (`self.K2_GetActorLocation`))
  (`self.K2_DestroyActor`)
  (`|SpawnActorFromClass` "/Game/GameOff/Assets/Bone.Bone_C" (`KismetMathLibrary.MakeTransform` (`KismetMathLibrary.MakeVector` _returnvalue_x _returnvalue_y 80.0)) "Undefined" "OverrideRootScale" null null))

(fn `UserConstructionScript`)